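; BP_Level0 is a level-pass actor that reveals a configurable mesh, apparently a gold coin ("jinbi"), and flies it along a spline.
; The mesh is assigned in the construction script and hidden at BeginPlay.
; Tick polls the game instance's IsPass flag, then unhides the mesh and calls Play on a timeline.
; Each timeline update positions the mesh by spline distance, eases rotation toward TargetRotation with RInterpTo and applies Rate as play rate.
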(event `self.ReceiveBeginPlay`
  (`SceneComponent.SetHiddenInGame` (`self.StaticMesh`) true false))

(event `self.ReceiveTick`
  (params (DeltaSeconds :type "Float (single-precision)"))
  (if (`/Game/UI/BluePrint/LM_GameInstance.IsPass` (`/Game/UI/BluePrint/FunctionLibrary.GetMyGameInstance`))
    (`SceneComponent.SetHiddenInGame` (`self.StaticMesh`) false false)
    (bind (_direction _move) (`Timeline|Level0_jinbi`)
      (:`Update`
        (`SceneComponent.K2_SetWorldLocation` (`self.StaticMesh`) (`SplineComponent.GetLocationAtDistanceAlongSpline` (`self.Spline`) (* _move (`SplineComponent.GetSplineLength` (`self.Spline`))) "World") false false)
        (`SceneComponent.K2_SetWorldRotation` (`self.StaticMesh`) (`KismetMathLibrary.RInterpTo` (`SceneComponent.K2_GetComponentRotation` (`self.StaticMesh`)) (`self.TargetRotation`) (`GameplayStatics.GetWorldDeltaSeconds`) 1.0) false false)
        (`TimelineComponent.SetPlayRate` (`self.Level0_jinbi`) (`self.Rate`))))))

(fn `UserConstructionScript`
  (`StaticMeshComponent.SetStaticMesh` (`self.StaticMesh`) (`self.NewMesh`)))