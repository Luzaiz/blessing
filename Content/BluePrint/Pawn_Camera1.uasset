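; Pawn_Camera1 is a camera pawn that provides mouse-driven view rotation and zoom.
; Holding the left mouse button sets a flag that lets mouse X and Y feed controller yaw and pitch input, with pitch inverted.
; The mouse wheel zooms by stepping the SpringArm's target length by ArmSpeed, clamped between the Min and Max variables.
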(event `Key|MouseScrollUp`
  (params (Key :type "Key Structure"))
  (bind _springarm (`self.SpringArm`))
  ;[1 1 1] 缩放视图
  (:`Pressed`
    (set `SpringArmComponent.TargetArmLength` (`KismetMathLibrary.FClamp` (- (`SpringArmComponent.TargetArmLength` _springarm) (`self.ArmSpeed`)) (`self.Min`) (`self.Max`)) _springarm)))

(event `InputAxisKey|MouseX`
  (params (AxisValue :type "Float (single-precision)"))
  ;[1 1 1] 旋转视角
  (if (`self.MouseLeft`)
    (`self.AddControllerYawInput` AxisValue)))

(event `InputAxisKey|MouseY`
  (params (AxisValue :type "Float (single-precision)"))
  ;[1 1 1] 旋转视角
  (if (`self.MouseLeft`)
    (`self.AddControllerPitchInput` (* AxisValue -1.0))))

(event `Key|MouseScrollDown`
  (params (Key :type "Key Structure"))
  (bind _springarm (`self.SpringArm`))
  ;[1 1 1] 缩放视图
  (:`Pressed`
    (set `SpringArmComponent.TargetArmLength` (`KismetMathLibrary.FClamp` (+ (`SpringArmComponent.TargetArmLength` _springarm) (`self.ArmSpeed`)) (`self.Min`) (`self.Max`)) _springarm)))

(event `Key|LeftMouseButton`
  (params (Key :type "Key Structure"))
  ;[1 1 1] 鼠标左键功能
  (:`Pressed`
    (set `self.MouseLeft` true))
  (:`Released`
    (set `self.MouseLeft` false)))

(fn `UserConstructionScript`)