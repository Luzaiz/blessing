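; BP_Camera2 is a camera rig Blueprint that orbits and zooms through a SpringArm.
; BeginPlay sets the arm's starting pitch from DefaultCameraPitchValue.
; CE_CameraRotation adds scaled horizontal and vertical input to the arm's relative yaw and pitch, clamping pitch just short of vertical and holding roll at zero.
; CE_MouseWheel changes arm length by scaled input within caller-supplied nearest and farthest limits.
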(event `self.ReceiveBeginPlay`
  (`SceneComponent.K2_SetRelativeRotation` (`self.SpringArm`) (`KismetMathLibrary.MakeRotator` 0.0 (`self.DefaultCameraPitchValue`)) false false))

(event `self.ReceiveTick`
  (params (DeltaSeconds :type "Float (single-precision)")))

(event `CE_CameraRotation`
  (params (`水平旋转参数` :type "Float (double-precision)") (`垂直旋转参数` :type "Float (double-precision)") (`旋转差值` :type "Float (double-precision)"))
  ;[1 1 1] 计算Yaw
  (`SceneComponent.K2_SetRelativeRotation` (`self.SpringArm`) (`KismetMathLibrary.MakeRotator` 0.0 (.pitch (`SceneComponent.RelativeRotation` (`self.SpringArm`))) (+ (.yaw (`SceneComponent.RelativeRotation` (`self.SpringArm`))) (* `水平旋转参数` `旋转差值`))) false false)
  (`SceneComponent.K2_SetRelativeRotation` (`self.SpringArm`) (`KismetMathLibrary.MakeRotator` 0.0 (`KismetMathLibrary.ClampAngle` (+ (* `垂直旋转参数` `旋转差值`) (.pitch (`SceneComponent.RelativeRotation` (`self.SpringArm`)))) -89.900002 89.900002) (.yaw (`SceneComponent.RelativeRotation` (`self.SpringArm`)))) false false))

(event `CE_MouseWheel`
  (params (`参数` :type "Float (double-precision)") (`差值` :type "Float (double-precision)") (`最近` :type "Float (double-precision)") (`最远` :type "Float (double-precision)"))
  (bind _springarm (`self.SpringArm`))
  (set `SpringArmComponent.TargetArmLength` (`KismetMathLibrary.FClamp` (+ (* `参数` `差值`) (`SpringArmComponent.TargetArmLength` _springarm)) `最近` `最远`) _springarm))

(fn `UserConstructionScript`)