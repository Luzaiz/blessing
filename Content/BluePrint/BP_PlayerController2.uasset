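; Player controller that drives a BP_Camera2 actor found in the level, using it as the view target with the mouse cursor shown.
; Each tick, unless paused, it forwards axis input for wheel zoom and, through a gate held open by left mouse, drag rotation.
; Tab toggles a pause flag and widget, marked buggy: widget creation and SetGamePaused are disconnected, so the game itself never pauses.
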(event `self.ReceiveBeginPlay`
  (`|ExecutionSequence`
    (:`then_1`
      ;[1 1 1] 获取摄像机视角和鼠标显示
      (bind _returnvalue (`GameplayStatics.GetActorOfClass` "/Game/BluePrint/BP_Camera2.BP_Camera2_C"))
      (bind _output_get (set `self.BP_Camera` _returnvalue))
      (`self.SetViewTargetWithBlend` _output_get)
      (set `self.bShowMouseCursor` true))))

(event `Key|Tab`
  (params (Key :type "Key Structure"))
  ;[1 1 1] TAB打开暂停界面并暂停游戏（先别用有bug）
  (:`Pressed`
    (if (`self.IsGamePause`)
      (`self.GameContinue`)
      (else
        (`self.GamePause`)))))

(event `GamePause`
  ;[1 1 1] TAB打开暂停界面并暂停游戏（先别用有bug）
  (`UserWidget.AddToViewport` (`self.UI_Pause`) 0)
  (set `self.IsGamePause` true))

(event `GameContinue`
  ;[1 1 1] TAB打开暂停界面并暂停游戏（先别用有bug）
  (`Widget.RemoveFromParent` (`self.UI_Pause`))
  (set `self.IsGamePause` false))

(event `self.ReceiveTick`
  (params (DeltaSeconds :type "Float (single-precision)"))
  (`|ExecutionSequence`
    (:`then_0`
      ;[1 1 1] 移动视角
      (if (not (`self.IsGamePause`))
        (`|ExecutionSequence`
          (:`then_0`
            ;;[1 1 1] 鼠标x轴移动旋转摄像机水平
            (`/Engine/EditorBlueprintResources/StandardMacros.Gate` true :!label _label
              (:`Exit`
                (`/Game/BluePrint/BP_Camera2.CE_CameraRotation` (`self.BP_Camera`) (`self.GetInputAxisKeyValue`) (`self.GetInputAxisKeyValue`) 4.0))))
          (:`then_1`
            (`/Game/BluePrint/BP_Camera2.CE_MouseWheel` (`self.BP_Camera`) (`self.GetInputAxisKeyValue`) -30.0 500.0 700.0)))))))

(event `Key|LeftMouseButton`
  (params (Key :type "Key Structure"))
  ;[1 1 1] 移动视角
  ;;[1 1 1] 鼠标x轴移动旋转摄像机水平
  (:`Pressed`
    (goto _label :!via `Open`))
  (:`Released`
    (goto _label :!via `Close`)))

(fn `UserConstructionScript`)